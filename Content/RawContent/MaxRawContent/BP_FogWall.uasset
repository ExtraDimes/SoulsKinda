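; Fog wall actor that dissolves and stops blocking when the BP_MK_Third_Person player overlaps its trigger box.
; The overlap calls OpenDoorEvent only if HasAlreadyOverlapped is already true, then redundantly sets that flag true.
; OpenDoorEvent creates a dynamic scrolling-fog material on FogWall, and a timeline drives its LerpValue parameter.
; When the timeline finishes, the root component deactivates and FogWall collision is disabled.
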(event OnComponentBeginOverlap(BoxCollide)
  (params (OverlappedComponent :type Primitive%20Component%20Object%20Reference) (OtherActor :type Actor%20Object%20Reference) (OtherComp :type Primitive%20Component%20Object%20Reference) (OtherBodyIndex :type Integer) (bFromSweep :type Boolean) (SweepResult :type Hit%20Result%20Structure%20%28by%20ref%29))
  (Utilities|Casting|CastToBP_MK_Third_Person OtherActor)
  (if (Variables|Default|GetHasAlreadyOverlapped)
    (Variables|Default|SetHasAlreadyOverlapped true)
    (CallFunction|OpenDoorEvent)))

(event Custom|OpenDoorEvent
  (bind _returnvalue (Rendering|Material|CreateDynamicMaterialInstance (Variables|Default|GetFogWall) 0 "/Game/RawContent/MaxRawContent/Materials/MS_ScrollingFog.MS_ScrollingFog" "None" :!class /Script/Engine.PrimitiveComponent))
  (Variables|Default|SetDynamicMaterial _returnvalue)
  (bind _lerpvalue (Timeline|LerpValueTimeline Play)
    (:Update
      (Rendering|Material|SetScalarParameterValue (Variables|Default|GetDynamicMaterial) "LerpValue" _lerpvalue :!class /Script/Engine.MaterialInstanceDynamic))
    (:Finished
      (Components|Activation|Deactivate (Variables|Default|GetDefaultSceneRoot))
      (Collision|SetCollisionEnabled (Variables|Default|GetFogWall) "NoCollision"))))

(fn ConstructionScript)