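; BP_WeaponPickable is a world weapon pickup driven by a WeaponData variable.
; The construction script sets its static mesh from WeaponData.
; When an actor implementing BPI_Interact overlaps PickupTrigger, it sends that actor a pickup message with WeaponData, plays an attenuated pickup sound and destroys itself.
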(event OnComponentBeginOverlap(PickupTrigger)
  (params (OverlappedComponent :type Primitive%20Component%20Object%20Reference) (OtherActor :type Actor%20Object%20Reference) (OtherComp :type Primitive%20Component%20Object%20Reference) (OtherBodyIndex :type Integer) (bFromSweep :type Boolean) (SweepResult :type Hit%20Result%20Structure%20%28by%20ref%29))
  (if (Utilities|DoesObjectImplementInterface OtherActor "/Game/RawContent/Medhank_RawContent/Blueprints/Weapons/BPI_Interact.BPI_Interact_C")
    (Class|BPIInteract|PickupWeapon(Message) OtherActor (Variables|Default|GetweaponData))
    (Audio|PlaySoundatLocation "/Game/RawContent/Medhank_RawContent/Audio/Sounds/ItemGet.ItemGet" "0, 0, 0" "0, 0, 0" 0.8 1.0 0.0 "/Game/RawContent/Medhank_RawContent/Audio/SA_Character.SA_Character" 0 0 0)
    (Actor|DestroyActor)))

(event EventBeginPlay)

(event Collision|EventActorBeginOverlap
  (params (OtherActor :type Actor%20Object%20Reference)))

(event EventTick
  (params (DeltaSeconds :type Float%20%28single-precision%29)))

(fn ConstructionScript
  (Components|StaticMesh|SetStaticMesh (Variables|Default|GetStaticMesh) (Variables|/Game/RawContent/Medhank_RawContent/Blueprints/Weapons/BP_DA_Weapon.BP_DA_Weapon_C|GetstaticMesh (Variables|Default|GetweaponData))))