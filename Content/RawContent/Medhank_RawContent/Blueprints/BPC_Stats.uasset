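; Actor component that tracks its owner's health stat and signals death.
; IncreaseValue takes a stat selector and an amount, then adds the amount to Health, clamped between zero and MaxHealth.
; At zero health it calls Die, which forwards DieMessage to the owning actor.
; It also updates a health progress bar, supplied through SetHealthProgressBar, with the current health fraction when that bar is valid.
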(event Custom|Die
  (Class|BPIDamage|Die(Message) (Components|GetOwner)))

(event Custom|Set%20Health%20Progress%20Bar
  (params (Health%20Progress%20Bar :type Progress%20Bar%20Object%20Reference))
  (Variables|Default|SetHealth%20Progress%20Bar Health%20Progress%20Bar))

(fn IncreaseValue
  (params (stat :type E_Stats%20Enum :default "NewEnumerator0") (Value :type Float%20%28double-precision%29))
  (switch Utilities|FlowControl|Switch|SwitchonE_Stats stat
    (:NewEnumerator0
      (Variables|Default|SetHealth (Math|Float|Clamp(Float) (+ (Variables|Default|GetHealth) Value) 0.0 (Variables|Default|GetMaxHealth)))
      (Utilities|FlowControl|Sequence
        (:then_0
          (if (<= (Variables|Default|GetHealth) 0.0)
            (CallFunction|Die)))
        (:then_1
          (bind _health_progress_bar (Variables|Default|GetHealth%20Progress%20Bar)
            (:then
              (Progress|SetPercent _health_progress_bar (/ (Variables|Default|GetHealth) (Variables|Default|GetMaxHealth))))
            (:else)))))))